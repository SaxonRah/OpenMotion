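; UBIKHelpers is a Blueprint set of helper functions for UBIK, covering debug drawing and rotation math.
; DrawAxes draws a transform's forward, right and up axes as red, green and blue debug arrows, with an optional sphere at its location.
; FindBetweenNormalsBP builds a normalized quaternion from the dot and cross products of two vectors and returns it as a rotator, using a perpendicular-axis fallback when they are nearly opposite.
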(fn DrawAxes
  (params (Transform :type Transform) (ArrowLength :type Float%20%28single-precision%29) (DrawSphere :type Boolean) (SphereRadius :type Float%20%28single-precision%29) (SphereColor :type Linear%20Color%20Structure :default "(R=1.000000,G=1.000000,B=1.000000,A=1.000000)"))
  (bind _output_get (LocalVariables|SetLocation (.location Transform)))
  (bind _output_get_2 (LocalVariables|SetRotation (.rotation Transform)))
  (Rendering|Debug|DrawDebugArrow 0 _output_get (+ _output_get (* (Math|Vector|GetForwardVector _output_get_2) ArrowLength)) 0.0 "(R=1.000000,G=0.000000,B=0.000000,A=1.000000)" 0.0 0.5)
  (Rendering|Debug|DrawDebugArrow 0 (LocalVariables|GetLocation) (+ (LocalVariables|GetLocation) (* (Math|Vector|GetRightVector (LocalVariables|GetRotation)) ArrowLength)) 0.0 "(R=0.000000,G=1.000000,B=0.000000,A=1.000000)" 0.0 0.5)
  (Rendering|Debug|DrawDebugArrow 0 (LocalVariables|GetLocation) (+ (LocalVariables|GetLocation) (* (Math|Vector|GetUpVector (LocalVariables|GetRotation)) ArrowLength)) 0.0 "(R=0.000000,G=0.000000,B=1.000000,A=1.000000)" 0.0 0.5)
  (if DrawSphere
    (Rendering|Debug|DrawDebugSphere 0 (LocalVariables|GetLocation) SphereRadius 12 SphereColor)))

(fn FindBetweenNormalsBP
  (params (A :type Vector) (B :type Vector))
  (bind _returnvalue (Math|Float|Absolute(Float) (.y A)))
  (bind _returnvalue_2 (Math|Float|Absolute(Float) (.x A)))
  (bind _returnvalue_3 (Math|Vector|CrossProduct A B))
  (bind _returnvalue_4 (* (.z A) -1.0))
  (bind _returnvalue_5 (* (.z A) -1.0))
  (bind _returnvalue_6 (> _returnvalue_2 _returnvalue))
  (bind _returnvalue_7 (Math|Vector|SelectVector (Math|Vector|MakeVector _returnvalue_5 0.0 (.x A)) (Math|Vector|MakeVector 0.0 _returnvalue_4 (.y A)) _returnvalue_6))
  (bind _output_get (LocalVariables|SetW (+ (Math|Vector|DotProduct A B) 1.0)))
  (if (> _output_get 1e-06)
    (return (Class|KismetMathLibrary|QuatRotator (Class|KismetMathLibrary|QuatNormalized (Utilities|Struct|MakeQuat (.x _returnvalue_3) (.y _returnvalue_3) (.z _returnvalue_3) (LocalVariables|GetW)) 0.0001)))
    (else
      (LocalVariables|SetW 0.0)
      (return (Class|KismetMathLibrary|QuatRotator (Class|KismetMathLibrary|QuatNormalized (Utilities|Struct|MakeQuat (.x _returnvalue_7) (.y _returnvalue_7) (.z _returnvalue_7) (LocalVariables|GetW)) 0.0001))))))